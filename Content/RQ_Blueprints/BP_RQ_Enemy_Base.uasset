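; Base enemy Blueprint that can be targeted by a lock-on and takes damage until death.
; SetTargetedStatus stores the targeted flag and shows or hides the lock-on reticle, with a debug print still in place.
; TakeRQDamage reduces clamped health, which starts full on BeginPlay, and plays a hit montage while alive.
; At zero health it disables capsule collision, plays the death montage, then switches the mesh to a physics ragdoll on completion.
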(event `SetTargetedStatus_1`
  (params (Status :type Boolean))
  (bind _lockonreticle (`self.LockOnreticle`))
  ; Lock
  (`KismetSystemLibrary.PrintString` "gOT")
  (bind _output_get (set `self.IsTargeted` Status))
  (if _output_get
    (`SceneComponent.SetVisibility` _lockonreticle true false)
    (else
      (`SceneComponent.SetVisibility` _lockonreticle false false))))

(event `/Game/RQ_Blueprints/Framework/BP_RQ_Damageable.TakeRQDamage`
  (params (DamageAmount :type "Float (double-precision)") (HitLocation :type "Vector Structure") (Attacker :type "Actor Object Reference"))
  (bind _mesh (`self.Mesh`))
  ; EnemyHP and Anim
  (set `self.CurrentHealth` (`KismetMathLibrary.FClamp` (- (`self.CurrentHealth`) DamageAmount) 0.0 (`self.MaxHealth`)))
  (if (<= (`self.CurrentHealth`) 0.0)
    ;; Disable actor capsule and trigger mesh physical simulation for death ragdoll
    (`PrimitiveComponent.SetCollisionEnabled` (`self.CapsuleComponent`) "NoCollision")
    (`|PlayMontage` null (`self.DeathMontage`)
      (:`OnCompleted`
        (`PrimitiveComponent.SetCollisionProfileName` _mesh "Ragdoll" true)
        (`PrimitiveComponent.SetSimulatePhysics` _mesh true)))
    (else
      (`self.PlayAnimMontage` (`self.HitMontage`)))))

(event `self.ReceiveBeginPlay`
  ; EnemyHP and Anim
  (bind _output_get (set `self.MaxHealth` 100.0))
  (set `self.CurrentHealth` _output_get))

(fn `UserConstructionScript`)