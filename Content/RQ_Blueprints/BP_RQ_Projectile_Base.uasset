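; Base projectile Blueprint that handles impact and cleanup, leaving the impact effect itself to an empty HandleImpact function, apparently for children to override.
; BeginPlay sets a lifespan from a variable.
; Any actor overlap spawns the impact emitter at the projectile, calls HandleImpact with Damage and the overlapped actor, then destroys the projectile.
; The impact sound plays at the world origin rather than the projectile's location.
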(event `self.ReceiveActorBeginOverlap`
  (params (OtherActor :type "Actor Object Reference"))
  (`GameplayStatics.SpawnEmitterAtLocation` (`self.ImpactVFX`) (`self.K2_GetActorLocation`))
  (`GameplayStatics.PlaySoundAtLocation` (`self.ImpactSFX`) (0.0 0.0 0.0) (struct) 1.0 1.0 0.0 null null null null)
  (`self.HandleImpact` (`self.Damage`) OtherActor)
  (`self.K2_DestroyActor`))

(event `self.ReceiveBeginPlay`
  (`self.SetLifeSpan` (`self.LifeSpan`)))

(fn `HandleImpact`
  (params (DamageAmount :type "Float (double-precision)") (HitActor :type "Actor Object Reference")))

(fn `UserConstructionScript`)