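; BP_RQ_Character is a player character with Souls-like camera-relative movement, sprint, jump and target lock-on.
; Enhanced Input events drive look and movement, with movement blocked while stunned.
; Lock-on toggles by sphere-overlapping targetable actors, choosing the best forward camera dot product, then interpolating control rotation toward it each Tick.
; Tick also tracks speed, acceleration and air time, and landing sends impact velocity and air time to the AnimInstance.
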(event `EnhancedInput|/Game/Input/Actions/IA_MouseLook`
  (params (ActionValue :type "Vector2D Structure") (ElapsedSeconds :type "Float (double-precision)") (TriggeredSeconds :type "Float (double-precision)") (InputAction :type "InputAction Object Reference" :default "/Game/Input/Actions/IA_MouseLook.IA_MouseLook"))
  ; Split 2D input into Yaw (Horizontal) and Pitch (Vertical) for camera control
  (:`Triggered`
    (`self.AddControllerYawInput` ActionValue_X)
    (`self.AddControllerPitchInput` ActionValue_Y)))

(event `EnhancedInput|/Game/Input/Actions/IA_Look`
  (params (ActionValue :type "Vector2D Structure") (ElapsedSeconds :type "Float (double-precision)") (TriggeredSeconds :type "Float (double-precision)") (InputAction :type "InputAction Object Reference" :default "/Game/Input/Actions/IA_Look.IA_Look"))
  ; Split 2D input into Yaw (Horizontal) and Pitch (Vertical) for camera control
  (:`Triggered`
    (`self.AddControllerYawInput` ActionValue_X)
    (`self.AddControllerPitchInput` ActionValue_Y)))

(event `EnhancedInput|/Game/Input/Actions/IA_Move`
  (params (ActionValue :type "Vector2D Structure") (ElapsedSeconds :type "Float (double-precision)") (TriggeredSeconds :type "Float (double-precision)") (InputAction :type "InputAction Object Reference" :default "/Game/Input/Actions/IA_Move.IA_Move"))
  (bind _returnvalue (`KismetMathLibrary.MakeRotator` 0.0 0.0 (.yaw (`self.GetControlRotation`))))
  ; Souls-like Movement: Decouple Actor Rotation from Camera-Relative Direction
  (:`Triggered`
    (if (not (`self.bIsStunned`))
      (`self.AddMovementInput` (`KismetMathLibrary.GetForwardVector` _returnvalue) ActionValue_Y)
      (`self.AddMovementInput` (`KismetMathLibrary.GetRightVector` _returnvalue) ActionValue_X))))

(event `EnhancedInput|/Game/Input/Actions/IA_Sprint`
  (params (ActionValue :type Boolean) (ElapsedSeconds :type "Float (double-precision)") (TriggeredSeconds :type "Float (double-precision)") (InputAction :type "InputAction Object Reference" :default "/Game/Input/Actions/IA_Sprint.IA_Sprint"))
  ; Sprint
  (:`Triggered`
    (set `self.bIsSprinting` true)
    (set `CharacterMovementComponent.MaxWalkSpeed` 550.0 (`self.CharacterMovement`)))
  (:`Completed`
    (set `self.bIsSprinting` false)
    (set `CharacterMovementComponent.MaxWalkSpeed` 400.0 (`self.CharacterMovement`))))

(event `EnhancedInput|/Game/Input/Actions/IA_Jump`
  (params (ActionValue :type Boolean) (ElapsedSeconds :type "Float (double-precision)") (TriggeredSeconds :type "Float (double-precision)") (InputAction :type "InputAction Object Reference" :default "/Game/Input/Actions/IA_Jump.IA_Jump"))
  ; Sprint
  (:`Started`
    (`self.Jump`)))

(event `self.ReceiveBeginPlay`
  ; Initialize Enhanced Input & Mapping Context                                                                                      (Bootstrap: Register Enhanced Input Mapping Context on BeginPlay)
  (`EnhancedInputSubsystemInterface.AddMappingContext` (pcsubsystem `EnhancedInputLocalPlayerSubsystem` (`GameplayStatics.GetPlayerController` 0)) "/Game/Input/IMC_Default.IMC_Default" 0 (struct))
  (set `CharacterMovementComponent.MaxWalkSpeed` 400.0 (`self.CharacterMovement`)))

(event `self.ReceiveTick`
  (params (DeltaSeconds :type "Float (single-precision)"))
  (bind _charactermovement (`self.CharacterMovement`))
  (`|ExecutionSequence`
    (:`then_0`
      ; Get acceleration, speed, in air time
      (set `self.Speed` (`KismetMathLibrary.VSize` (`self.GetVelocity` (`ActorComponent.GetOwner` _charactermovement))))
      (set `self.bIsAccelerating` (> (`KismetMathLibrary.VSize` (`CharacterMovementComponent.GetCurrentAcceleration` _charactermovement)) 0.0))
      (set `self.bIsInAir` (`NavMovementComponent.IsFalling` (`self.CharacterMovement`)))
      (if (`self.bIsInAir`)
        (set `self.AirTime` (+ DeltaSeconds (`self.AirTime`)))))
    (:`then_1`
      (`/Engine/EditorBlueprintResources/StandardMacros.IsValid` (`self.CurrentLockedTarget`)
        (:`Is Valid`
          (`Controller.SetControlRotation` (`GameplayStatics.GetPlayerController` 0) (`KismetMathLibrary.RInterpTo` (`self.GetControlRotation`) (`KismetMathLibrary.FindLookAtRotation` (`self.K2_GetActorLocation`) (`self.K2_GetActorLocation` (`self.CurrentLockedTarget`))) (`GameplayStatics.GetWorldDeltaSeconds`) 10.0)))))))

(event `self.OnLanded`
  (params (Hit :type "HitResult Structure (by ref)"))
  (bind (_velocity_x _velocity_y _velocity_z) (`KismetMathLibrary.BreakVector` (`MovementComponent.Velocity` (`self.CharacterMovement`))))
  ; transmit Heavyland Signal
  (message `/Game/RQ_Blueprints/BPI_RQ_PlayerAnimSignals.OnHeavyLandSignal` (`SkeletalMeshComponent.GetAnimInstance` (`self.Mesh`)) _velocity_z (`self.AirTime`)))

(event `EnhancedInput|/Game/Input/Actions/IA_Target`
  (params (ActionValue :type Boolean) (ElapsedSeconds :type "Float (double-precision)") (TriggeredSeconds :type "Float (double-precision)") (InputAction :type "InputAction Object Reference" :default "/Game/Input/Actions/IA_Target.IA_Target"))
  ; Lock
  (:`Started`
    (`/Engine/EditorBlueprintResources/StandardMacros.IsValid` (`self.CurrentLockedTarget`)
      (:`Is Valid`
        (message `/Game/RQ_Blueprints/BPI_RQ_Targetable.SetTargetedStatus` (`self.CurrentLockedTarget`) false)
        (set `self.CurrentLockedTarget` null))
      (:`Is Not Valid`
        (set `self.Best Target` null)
        (set `self.MaxDotProduct` -1.0)
        (bind _outactors (`KismetSystemLibrary.SphereOverlapActors` (`self.K2_GetActorLocation`) 1500.0 (`|MakeArray` "ObjectTypeQuery3" "ObjectTypeQuery2" :!type "EObjectTypeQuery Enum") "/Game/RQ_Blueprints/BP_TargetableBase.BP_TargetableBase_C"))
        (`KismetSystemLibrary.PrintString` (`KismetStringLibrary.Conv_IntToString` (`KismetArrayLibrary.Array_Length` _outactors)))
        (for _array_element _outactors
          (message `/Game/RQ_Blueprints/BPI_RQ_Targetable.IsTargetable?` _array_element false)
          (bind _returnvalue (`KismetMathLibrary.Dot_VectorVector` (`SceneComponent.GetForwardVector` (`self.Camera`)) (`KismetMathLibrary.Normal` (- (`self.K2_GetActorLocation` _array_element) (`SceneComponent.K2_GetComponentLocation` (`self.Camera`))))))
          (`KismetSystemLibrary.PrintString` (`KismetStringLibrary.Conv_DoubleToString` _returnvalue))
          (if (> _returnvalue (`self.MaxDotProduct`))
            (bind _asbp_targetable_base (cast `/Game/RQ_Blueprints/BP_TargetableBase` _array_element))
            (bind _output_get (set `self.MaxDotProduct` _returnvalue))
            (if (> _output_get 0.1)
              (bind _output_get_2 (set `self.Best Target` _asbp_targetable_base)))))
        (`/Engine/EditorBlueprintResources/StandardMacros.IsValid` (`self.Best Target`)
          (:`Is Valid`
            (bind _output_get_3 (set `self.CurrentLockedTarget` _output_get_2))
            (message `/Game/RQ_Blueprints/BPI_RQ_Targetable.SetTargetedStatus` _output_get_3 true)
            (`KismetSystemLibrary.PrintString` (`KismetSystemLibrary.GetDisplayName` _output_get_3)))
          (:`Is Not Valid`
            (`KismetSystemLibrary.PrintString` "Hello")))))))

(fn `UserConstructionScript`)