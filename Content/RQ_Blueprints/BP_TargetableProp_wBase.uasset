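; BP_TargetableProp_wBase is a prop that can be locked onto and takes damage.
; SetTargetedStatus stores the targeted flag, toggles the LockOnreticle's visibility and prints a debug string.
; BeginPlay sets health to full; TakeRQDamage subtracts clamped damage and, while health remains, calls TakeRQDamage again with a zero hit location.
; IsTargetable and CheckShouldUnlock are empty stubs, and zero health triggers nothing here.
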(event `/Game/RQ_Blueprints/Framework/BPI_RQ_Targetable.SetTargetedStatus`
  (params (Status :type Boolean))
  (bind _lockonreticle (`self.LockOnreticle`))
  ; Lock
  (`KismetSystemLibrary.PrintString` "gOT")
  (bind _output_get (set `self.IsTargeted` Status))
  (if _output_get
    (`SceneComponent.SetVisibility` _lockonreticle true false)
    (else
      (`SceneComponent.SetVisibility` _lockonreticle false false))))

(event `/Game/RQ_Blueprints/Framework/BP_RQ_Damageable.TakeRQDamage`
  (params (DamageAmount :type "Float (double-precision)") (HitLocation :type "Vector Structure") (Attacker :type "Actor Object Reference"))
  (set `self.CurrentHealth` (`KismetMathLibrary.FClamp` (- (`self.CurrentHealth`) DamageAmount) 0.0 (`self.MaxHealth`)))
  (if (not (<= (`self.CurrentHealth`) 0.0))
    (`self.TakeRQDamage` DamageAmount)))

(event `self.ReceiveBeginPlay`
  (bind _output_get (set `self.MaxHealth` 100.0))
  (set `self.CurrentHealth` _output_get))

(fn `IsTargetable?`
  (params (Result :type Boolean))
  (return))

(fn `UserConstructionScript`)